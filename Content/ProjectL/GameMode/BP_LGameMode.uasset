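; Game mode for a boss fight that runs a gimmick phase and handles player and boss death.
; When Gimmic is set, Tick waits through a delay, broadcasts the state, then spawns balls, a bar and looping randomly sized floor hazards.
; Once GimmicPlayed is set, which is never reset here, EndGimmic accumulates time to clear the phase and floor timer.
; Death flags pause the game and show the matching HUD screen.
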(event EventBeginPlay)

(event EventTick
  (params (DeltaSeconds :type Float%20%28single-precision%29))
  (bind _gimmic (Variables|Default|GetGimmic))
  (Utilities|FlowControl|Sequence
    (:then_0
      ;[0.15 0.15 0.15 0.5] 기믹 관련
      (if (Variables|Default|GetGimmicPlayed)
        (CallFunction|EndGimmic DeltaSeconds)
        (elif _gimmic
          (Utilities|FlowControl|Delay 12.0)
          (Default|CallEventDispatcherIsGimmic _gimmic)
          (CallFunction|StartGimmic _gimmic))))
    (:then_1
      (if (Variables|Default|GetPlayerDied)
        (Game|SetGamePaused true)
        (bind _asbp_hud (Utilities|Casting|CastToBP_Hud (HUD|GetHUD (Game|GetPlayerController 0))))
        (Default|PlayerDie (Variables|/Game/UI/BP_Hud.BP_Hud_C|GetHudWidget _asbp_hud))
        (elif (Variables|Default|GetBossDied)
          (Utilities|FlowControl|Delay 1.0)
          (Game|SetGamePaused true)
          (bind _asbp_hud_2 (Utilities|Casting|CastToBP_Hud (HUD|GetHUD (Game|GetPlayerController 0))))
          (Default|BossDie (Variables|/Game/UI/BP_Hud.BP_Hud_C|GetHudWidget _asbp_hud_2)))))))

(fn ConstructionScript)

(fn SpawnGimmicBall
  (Game|SpawnActorfromClass "/Game/ProjectL/GameMode/Gimmicmap/BP_GimmicBalls.BP_GimmicBalls_C" (Math|Transform|MakeTransform "0, 0, 0" "0, 0, 0" "1.000000,1.000000,1.000000") "Undefined" "MultiplyWithRoot" 0 0))

(fn SpawnFloor
  (if (Math|Random|RandomBool)
    (Game|SpawnActorfromClass "/Game/ProjectL/GameMode/Gimmicmap/BP_GimmicFloor.BP_GimmicFloor_C" (Math|Transform|MakeTransform "0.000000,0.000000,10.000000" "0, 0, 0" "30.000000,30.000000,1.000000") "Undefined" "MultiplyWithRoot" 0 0)
    (else
      (Game|SpawnActorfromClass "/Game/ProjectL/GameMode/Gimmicmap/BP_GimmicFloor.BP_GimmicFloor_C" (Math|Transform|MakeTransform "0.000000,0.000000,10.000000" "0, 0, 0" "42.000000,42.000000,1.000000") "Undefined" "MultiplyWithRoot" 0 0))))

(fn EndGimmic
  (params (B :type Float%20%28double-precision%29))
  (bind _output_get (Variables|Default|SetGimmicTime (+ (Variables|Default|GetGimmicTime) B)))
  (if (> _output_get 25.0)
    (bind _output_get_2 (Variables|Default|SetGimmic false))
    (Default|CallEventDispatcherIsGimmic _output_get_2)
    (Utilities|Time|ClearTimerbyFunctionName 0 "SpawnFloor")
    (Variables|Default|SetGimmicTime 0.0)))

(fn StartGimmic
  (params (IsGimmic :type Boolean))
  (CallFunction|SpawnGimmicBall)
  (Game|SpawnActorfromClass "/Game/ProjectL/GameMode/Gimmicmap/BP_GimmicBar.BP_GimmicBar_C" (Math|Transform|MakeTransform "0.000000,0.000000,10.000000" "0, 0, 0" "1.000000,1.000000,1.000000") "Undefined" "MultiplyWithRoot" 0 0)
  (Utilities|Time|SetTimerbyFunctionName 0 "SpawnFloor" 3.5 true)
  (Variables|Default|SetGimmicPlayed true))

(fn SpawnGimmicLoc
  (Game|SpawnActorfromClass "/Game/ProjectL/GameMode/Gimmicmap/BP_GimmicStartLocation.BP_GimmicStartLocation_C" (Math|Transform|MakeTransform "0.000000,0.000000,5.000000" "0, 0, 0" "65.000000,65.000000,10.000000") "Undefined" "MultiplyWithRoot" 0 0))